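; Player character Blueprint with camera-relative walking, mouse look and jumping.
; Tick polls all input: IA_Forward and IA_Right values drive movement along the control yaw, mouse delta turns the controller with inverted pitch delta, and a held Space bar triggers Jump.
; A looping timer started on BeginPlay calls LogMovementState to print height and vertical velocity for debugging.
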(event `self.ReceiveTick`
  (params (DeltaSeconds :type "Float (single-precision)"))
  (bind _returnvalue (`GameplayStatics.GetPlayerController` 0))
  (bind (_deltax _deltay) (`PlayerController.GetInputMouseDelta` _returnvalue))
  (bind _returnvalue_2 (`KismetMathLibrary.MakeRotator` 0.0 0.0 (.yaw (`Controller.GetControlRotation` _returnvalue))))
  (`self.AddMovementInput` self (`KismetMathLibrary.GetForwardVector` _returnvalue_2) (`|GetInputActionValue`) false)
  (`self.AddMovementInput` self (`KismetMathLibrary.GetRightVector` _returnvalue_2) (`|GetInputActionValue`) false)
  (`self.AddControllerYawInput` self _deltax)
  (`self.AddControllerPitchInput` self (- 0.0 _deltay))
  (if (`PlayerController.IsInputKeyDown` _returnvalue "SpaceBar")
    (`self.Jump` self)
    (else
      (`self.StopJumping` self))))

(event `self.ReceiveBeginPlay`
  (`KismetSystemLibrary.K2_SetTimer` self "LogMovementState" 1.0 true))

(fn `LogMovementState`
  (`KismetSystemLibrary.PrintString` (`KismetStringLibrary.Concat_StrStr` (`KismetStringLibrary.Concat_StrStr` (`KismetStringLibrary.Concat_StrStr` "CharState: locZ=" (`KismetStringLibrary.Conv_DoubleToString` (.z (`self.K2_GetActorLocation`)))) " velZ=") (`KismetStringLibrary.Conv_DoubleToString` (.z (`self.GetVelocity` self)))) false true (struct :`G` 0.66 :`B` 1.0 :`A` 1.0) 2.0))

(fn `UserConstructionScript`)