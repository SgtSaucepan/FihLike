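; BP_BaseGamemode is a game mode that swaps a spawned DefaultPawn for BP_FihlikeCharacter at runtime.
; Shortly after BeginPlay, a timer calls FixPawnClass, which spawns the character at the first DefaultPawn's location, has that pawn's controller possess it, and destroys the old pawn.
; If no DefaultPawn exists or it lacks a controller, the function re-arms the timer and retries without limit, printing debug messages.
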(event `self.ReceiveBeginPlay`
  (`KismetSystemLibrary.K2_SetTimer` self "FixPawnClass" 0.2))

(fn `FixPawnClass`
  (bind _outactors (`GameplayStatics.GetAllActorsOfClass` "/Script/Engine.DefaultPawn"))
  (if (> (`KismetArrayLibrary.Array_Length` _outactors) 0)
    (bind _output (`|GetArrayItem` _outactors))
    (bind _returnvalue (`Pawn.GetController` _output))
    (`/Engine/EditorBlueprintResources/StandardMacros.IsValid` _returnvalue
      (:`Is Valid`
        (bind _returnvalue_2 (`|SpawnActorFromClass` "/Game/Player/BP_FihlikeCharacter.BP_FihlikeCharacter_C" (`KismetMathLibrary.MakeTransform` (`self.K2_GetActorLocation` _output)) "AlwaysSpawn" "MultiplyWithRoot" null null))
        (`Controller.Possess` _returnvalue _returnvalue_2)
        (`self.K2_DestroyActor` _output)
        (`KismetSystemLibrary.PrintString` "FixPawnClass: replaced DefaultPawn with BP_FihlikeCharacter" false true (struct :`G` 0.66 :`B` 1.0 :`A` 1.0) 2.0))
      (:`Is Not Valid`
        (`KismetSystemLibrary.PrintString` "FixPawnClass: DefaultPawn has no controller yet, retrying" false true (struct :`G` 0.66 :`B` 1.0 :`A` 1.0) 2.0)
        (`KismetSystemLibrary.K2_SetTimer` self "FixPawnClass" 0.3)))
    (else
      (`KismetSystemLibrary.PrintString` "FixPawnClass: no DefaultPawn found, retrying" false true (struct :`G` 0.66 :`B` 1.0 :`A` 1.0) 2.0)
      (`KismetSystemLibrary.K2_SetTimer` self "FixPawnClass" 0.3))))

(fn `UserConstructionScript`)