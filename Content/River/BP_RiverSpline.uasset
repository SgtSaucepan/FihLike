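; River actor that procedurally lays out a flat, meandering spline river from a random seed.
; BeginPlay rebuilds the spline along local X, with Y drifting by accumulated per-index seeded random offsets scaled by meander settings.
; RegenerateRiver repeats that build and also places an instanced mesh at each point, scaled to segment length and river width.
; GetPointAtDistance returns the world transform at a distance along the spline.
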(event `self.ReceiveBeginPlay`
  (bind _meanderfrequency (`self.MeanderFrequency`))
  (bind _riversplinecomp (`self.RiverSplineComp`))
  (`SplineComponent.ClearSplinePoints` _riversplinecomp false)
  (set `self.LateralOffsetAccum` 0.0)
  (for _index (range (+ (- (`self.NumPoints`) 1) 1))
    (bind _returnvalue (+ (`self.LateralOffsetAccum`) (* (`KismetMathLibrary.RandomFloatInRangeFromStream` (`KismetMathLibrary.MakeRandomStream` (+ (`self.RandomSeed`) _index)) (- 0.0 _meanderfrequency) _meanderfrequency) (`self.MeanderStrength`))))
    (set `self.LateralOffsetAccum` _returnvalue)
    (`SplineComponent.AddSplinePoint` _riversplinecomp (`KismetMathLibrary.MakeVector` (* _index (`self.SegmentLength`)) _returnvalue) "Local" false))
  (`SplineComponent.UpdateSpline` _riversplinecomp))

(fn `GetPointAtDistance`
  (params (Distance :type "Float (double-precision)"))
  (returns (PointTransform :type "Transform Structure"))
  (return (`SplineComponent.GetTransformAtDistanceAlongSpline` (`self.RiverSplineComp`) Distance "World" false)))

(fn `RegenerateRiver`
  (bind _riversplinecomp (`self.RiverSplineComp`))
  (bind _numpoints (`self.NumPoints`))
  (bind _segmentlength (`self.SegmentLength`))
  (bind _meanderfrequency (`self.MeanderFrequency`))
  (bind _rivercubeism (`self.RiverCubeISM`))
  (`SplineComponent.ClearSplinePoints` _riversplinecomp false)
  (set `self.LateralOffsetAccum` 0.0)
  (for _index (range (+ (- _numpoints 1) 1))
    (bind _returnvalue (+ (`self.LateralOffsetAccum`) (* (`KismetMathLibrary.RandomFloatInRangeFromStream` (`KismetMathLibrary.MakeRandomStream` (+ (`self.RandomSeed`) _index)) (- 0.0 _meanderfrequency) _meanderfrequency) (`self.MeanderStrength`))))
    (set `self.LateralOffsetAccum` _returnvalue)
    (`SplineComponent.AddSplinePoint` _riversplinecomp (`KismetMathLibrary.MakeVector` (* _index _segmentlength) _returnvalue) "Local" false))
  (`SplineComponent.UpdateSpline` _riversplinecomp)
  (`InstancedStaticMeshComponent.ClearInstances` _rivercubeism)
  (for _index_2 (range (+ (- _numpoints 1) 1))
    (bind _returnvalue_2 (`SplineComponent.GetTransformAtSplinePoint` _riversplinecomp _index_2 "World" false))
    (`InstancedStaticMeshComponent.AddInstance` _rivercubeism (`KismetMathLibrary.MakeTransform` (.location _returnvalue_2) (.rotation _returnvalue_2) (`KismetMathLibrary.MakeVector` (/ _segmentlength 925.64) (/ (* (`self.RiverVisualWidth`) 2.0) 925.64) 1.0)) true)))

(fn `UserConstructionScript`)