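; Map generator that builds a procedural terrain mesh with a river at BeginPlay.
; It randomizes and regenerates BP_RiverSpline, then samples height per grid cell, blending sine-wave hills down to the riverbed by distance to the spline.
; Cells near the river form a sand section, the rest grass, both with collision.
; A delayed callback draws BP_GridManager's grid and line-traces the player onto the terrain, retrying until successful.
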(event `self.ReceiveBeginPlay`
  (bind _vertices (`self.Vertices`))
  (bind _triangles (`self.Triangles`))
  (bind _sandvertices (`self.SandVertices`))
  (bind _sandtriangles (`self.SandTriangles`))
  (bind _mapsize (`self.MapSize`))
  (bind _resolution (`self.Resolution`))
  (bind _terrainmesh (`self.TerrainMesh`))
  (bind _returnvalue (/ _mapsize 2.0))
  (bind _returnvalue_2 (/ _mapsize _resolution))
  (bind _outactors (`GameplayStatics.GetAllActorsOfClass` "/Game/River/BP_RiverSpline.BP_RiverSpline_C"))
  (bind _asbp_river_spline (cast `/Game/River/BP_RiverSpline` (`|GetArrayItem` _outactors)))
  (set `/Game/River/BP_RiverSpline.RandomSeed` (`KismetMathLibrary.RandomIntegerInRange` 0 999999) _asbp_river_spline)
  (`/Game/River/BP_RiverSpline.RegenerateRiver` _asbp_river_spline)
  (set `self.CachedRiverSpline` (`/Game/River/BP_RiverSpline.RiverSplineComp` _asbp_river_spline))
  (`KismetArrayLibrary.Array_Clear` _vertices)
  (`KismetArrayLibrary.Array_Clear` _triangles)
  (`KismetArrayLibrary.Array_Clear` _sandvertices)
  (`KismetArrayLibrary.Array_Clear` _sandtriangles)
  (for _index (range (+ (- _resolution 1) 1))
    (for _index_2 (range (+ (- _resolution 1) 1))
      (bind _returnvalue_3 (- (* _index_2 _returnvalue_2) _returnvalue))
      (bind _returnvalue_4 (- (* _index _returnvalue_2) _returnvalue))
      (bind (_height _riverfactor) (`self.SampleTerrain` (`KismetMathLibrary.Conv_IntToDouble` _returnvalue_3) (`KismetMathLibrary.Conv_IntToDouble` _returnvalue_4)))
      (bind _returnvalue_5 (- (* (+ _index_2 1) _returnvalue_2) _returnvalue))
      (bind (_height_2 _riverfactor_2) (`self.SampleTerrain` (`KismetMathLibrary.Conv_IntToDouble` _returnvalue_5) (`KismetMathLibrary.Conv_IntToDouble` _returnvalue_4)))
      (bind _returnvalue_6 (- (* (+ _index 1) _returnvalue_2) _returnvalue))
      (bind (_height_3 _riverfactor_3) (`self.SampleTerrain` (`KismetMathLibrary.Conv_IntToDouble` _returnvalue_3) (`KismetMathLibrary.Conv_IntToDouble` _returnvalue_6)))
      (bind (_height_4 _riverfactor_4) (`self.SampleTerrain` (`KismetMathLibrary.Conv_IntToDouble` _returnvalue_5) (`KismetMathLibrary.Conv_IntToDouble` _returnvalue_6)))
      (if (< (/ (+ (+ _riverfactor _riverfactor_2) (+ _riverfactor_3 _riverfactor_4)) 4.0) 0.6)
        (bind _returnvalue_7 (`KismetMathLibrary.MakeVector` (`KismetMathLibrary.Conv_IntToDouble` _returnvalue_3) (`KismetMathLibrary.Conv_IntToDouble` _returnvalue_4) _height))
        (bind _returnvalue_8 (`KismetArrayLibrary.Array_Add` _sandvertices _returnvalue_7))
        (bind _returnvalue_9 (`KismetMathLibrary.MakeVector` (`KismetMathLibrary.Conv_IntToDouble` _returnvalue_5) (`KismetMathLibrary.Conv_IntToDouble` _returnvalue_4) _height_2))
        (bind _returnvalue_10 (`KismetArrayLibrary.Array_Add` _sandvertices _returnvalue_9))
        (bind _returnvalue_11 (`KismetMathLibrary.MakeVector` (`KismetMathLibrary.Conv_IntToDouble` _returnvalue_3) (`KismetMathLibrary.Conv_IntToDouble` _returnvalue_6) _height_3))
        (bind _returnvalue_12 (`KismetArrayLibrary.Array_Add` _sandvertices _returnvalue_11))
        (bind _returnvalue_13 (`KismetMathLibrary.MakeVector` (`KismetMathLibrary.Conv_IntToDouble` _returnvalue_5) (`KismetMathLibrary.Conv_IntToDouble` _returnvalue_6) _height_4))
        (bind _returnvalue_14 (`KismetArrayLibrary.Array_Add` _sandvertices _returnvalue_13))
        (`KismetArrayLibrary.Array_Add` _sandtriangles _returnvalue_8)
        (`KismetArrayLibrary.Array_Add` _sandtriangles _returnvalue_12)
        (`KismetArrayLibrary.Array_Add` _sandtriangles _returnvalue_10)
        (`KismetArrayLibrary.Array_Add` _sandtriangles _returnvalue_10)
        (`KismetArrayLibrary.Array_Add` _sandtriangles _returnvalue_12)
        (`KismetArrayLibrary.Array_Add` _sandtriangles _returnvalue_14)
        (else
          (bind _returnvalue_15 (`KismetArrayLibrary.Array_Add` _vertices _returnvalue_7))
          (bind _returnvalue_16 (`KismetArrayLibrary.Array_Add` _vertices _returnvalue_9))
          (bind _returnvalue_17 (`KismetArrayLibrary.Array_Add` _vertices _returnvalue_11))
          (bind _returnvalue_18 (`KismetArrayLibrary.Array_Add` _vertices _returnvalue_13))
          (`KismetArrayLibrary.Array_Add` _triangles _returnvalue_15)
          (`KismetArrayLibrary.Array_Add` _triangles _returnvalue_17)
          (`KismetArrayLibrary.Array_Add` _triangles _returnvalue_16)
          (`KismetArrayLibrary.Array_Add` _triangles _returnvalue_16)
          (`KismetArrayLibrary.Array_Add` _triangles _returnvalue_17)
          (`KismetArrayLibrary.Array_Add` _triangles _returnvalue_18)))))
  (`ProceduralMeshComponent.CreateMeshSection_LinearColor` :`self` _terrainmesh :`Vertices` _vertices :`Triangles` _triangles :`bCreateCollision` true)
  (`ProceduralMeshComponent.CreateMeshSection_LinearColor` :`self` _terrainmesh :`SectionIndex` 1 :`Vertices` _sandvertices :`Triangles` _sandtriangles :`bCreateCollision` true)
  (`PrimitiveComponent.SetMaterial` _terrainmesh 0 "/Game/Materials/M_Grass.M_Grass")
  (`PrimitiveComponent.SetMaterial` _terrainmesh 1 "/Game/Materials/M_Sand.M_Sand")
  (bind _outactors_2 (`GameplayStatics.GetAllActorsOfClass` "/Game/Grid/BP_GridManager.BP_GridManager_C"))
  (bind _asbp_grid_manager (cast `/Game/Grid/BP_GridManager` (`|GetArrayItem` _outactors_2))
    (:`then`
      (set `self.CachedGridActor` _asbp_grid_manager)
      (`KismetSystemLibrary.K2_SetTimer` self "PostTerrainReady" 1.0))
    (:`CastFailed`
      (`KismetSystemLibrary.K2_SetTimer` self "PostTerrainReady" 1.0))))

(fn `FixPlayerPlacement`
  (bind _returnvalue (`GameplayStatics.GetPlayerCharacter` 0))
  (bind _returnvalue_2 (`self.K2_GetActorLocation` _returnvalue))
  (bind _charactermovement (`Character.CharacterMovement` _returnvalue))
  (`/Engine/EditorBlueprintResources/StandardMacros.IsValid` _returnvalue
    (:`Is Valid`
      (bind (_outhit _returnvalue_3) (`KismetSystemLibrary.LineTraceSingle` (`KismetMathLibrary.MakeVector` (.x _returnvalue_2) (.y _returnvalue_2) 20000.0) (`KismetMathLibrary.MakeVector` (.x _returnvalue_2) (.y _returnvalue_2) -5000.0) "TraceTypeQuery1" true))
      (`KismetSystemLibrary.PrintString` (`KismetStringLibrary.Concat_StrStr` (`KismetStringLibrary.Concat_StrStr` (`KismetStringLibrary.Concat_StrStr` "FixPlayer: playerZ=" (`KismetStringLibrary.Conv_DoubleToString` (.z _returnvalue_2))) " didHit=") (`KismetStringLibrary.Conv_BoolToString` _returnvalue_3)) false true (struct :`G` 0.66 :`B` 1.0 :`A` 1.0) 2.0)
      (if _returnvalue_3
        (bind (_bblockinghit _binitialoverlap _time _distance _location) (`GameplayStatics.BreakHitResult` _outhit))
        (`self.K2_SetActorLocation` _returnvalue (`KismetMathLibrary.MakeVector` (.x _returnvalue_2) (.y _returnvalue_2) (+ (.z _location) 100.0)) false true)
        (`MovementComponent.StopMovementImmediately` _charactermovement)
        (`CharacterMovementComponent.SetMovementMode` _charactermovement "MOVE_Walking" 0)
        (`KismetSystemLibrary.PrintString` (`KismetStringLibrary.Concat_StrStr` "FixPlayer: teleported, hitZ+100=" (`KismetStringLibrary.Conv_DoubleToString` (.z _location))) false true (struct :`G` 0.66 :`B` 1.0 :`A` 1.0) 2.0)
        (else
          (`KismetSystemLibrary.PrintString` "FixPlayer: trace missed, retrying" false true (struct :`G` 0.66 :`B` 1.0 :`A` 1.0) 2.0)
          (`KismetSystemLibrary.K2_SetTimer` self "FixPlayerPlacement" 0.3))))
    (:`Is Not Valid`
      (bind _outactors (`GameplayStatics.GetAllActorsOfClass` "/Script/Engine.Pawn"))
      (if (> (`KismetArrayLibrary.Array_Length` _outactors) 0)
        (`KismetSystemLibrary.PrintString` (`KismetStringLibrary.Concat_StrStr` "FixPlayer: pawn class=" (`KismetSystemLibrary.GetClassDisplayName` (`GameplayStatics.GetObjectClass` (`|GetArrayItem` _outactors)))) false true (struct :`G` 0.66 :`B` 1.0 :`A` 1.0) 2.0)
        (`KismetSystemLibrary.K2_SetTimer` self "FixPlayerPlacement" 0.3)
        (else
          (`KismetSystemLibrary.PrintString` "FixPlayer: no pawns exist at all" false true (struct :`G` 0.66 :`B` 1.0 :`A` 1.0) 2.0)
          (`KismetSystemLibrary.K2_SetTimer` self "FixPlayerPlacement" 0.3))))))

(fn `PostTerrainReady`
  (bind _cachedgridactor (`self.CachedGridActor`))
  (`/Engine/EditorBlueprintResources/StandardMacros.IsValid` _cachedgridactor
    (:`Is Valid`
      (`/Game/Grid/BP_GridManager.DrawGrid` _cachedgridactor)
      (`self.FixPlayerPlacement`))
    (:`Is Not Valid`
      (`self.FixPlayerPlacement`))))

(fn `SampleTerrain`
  (params (LocalX :type "Float (double-precision)") (LocalY :type "Float (double-precision)"))
  (returns (Height :type "Float (double-precision)") (RiverFactor :type "Float (double-precision)"))
  (bind _returnvalue (`self.K2_GetActorLocation`))
  (bind _noisefrequency (`self.NoiseFrequency`))
  (bind _cachedriverspline (`self.CachedRiverSpline`))
  (bind _returnvalue_2 (+ (.x _returnvalue) LocalX))
  (bind _returnvalue_3 (+ (.y _returnvalue) LocalY))
  (bind _returnvalue_4 (`SplineComponent.GetLocationAtSplineInputKey` _cachedriverspline (`SplineComponent.FindInputKeyClosestToWorldLocation` _cachedriverspline (`KismetMathLibrary.MakeVector` _returnvalue_2 _returnvalue_3)) "World"))
  (bind _returnvalue_5 (- _returnvalue_3 (.y _returnvalue_4)))
  (bind _returnvalue_6 (- _returnvalue_2 (.x _returnvalue_4)))
  (bind _returnvalue_7 (`KismetMathLibrary.FClamp` (/ (- (`KismetMathLibrary.Sqrt` (+ (* _returnvalue_6 _returnvalue_6) (* _returnvalue_5 _returnvalue_5))) (`self.RiverWidth`)) (`self.RiverBankSmoothness`))))
  (return (`KismetMathLibrary.Lerp` (- 0.0 (`self.RiverDepth`)) (* (/ (+ (`KismetMathLibrary.DegSin` (* LocalX (* _noisefrequency 0.037))) (`KismetMathLibrary.DegSin` (* LocalY (* _noisefrequency 0.053)))) 2.0) (`self.HillHeight`)) _returnvalue_7) _returnvalue_7))

(fn `UserConstructionScript`)