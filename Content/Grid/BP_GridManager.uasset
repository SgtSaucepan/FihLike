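; Grid manager actor that maps world locations to cells on an XY grid anchored at its location and tracks which cells are occupied.
; Conversion functions return cell indices or cell centers, and occupancy is stored in OccupiedCells under "X,Y" string keys.
; When ShowGridInGame is set, BeginPlay draws flat debug lines at actor height.
; DrawGrid, uncalled in this Blueprint, draws a terrain-following version using downward line traces at cell corners.
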(event `self.ReceiveBeginPlay`
  (bind _returnvalue (`self.K2_GetActorLocation`))
  (bind _linearcolor (make `LinearColor` 1.0 1.0 1.0 1.0))
  (bind _cellsize (`self.CellSize`))
  (bind _gridextentx (`self.GridExtentX`))
  (bind _gridextenty (`self.GridExtentY`))
  (if (`self.bShowGridInGame`)
    (for _index (range (+ (- (+ _gridextentx 1) 1) 1))
      (bind _returnvalue_2 (+ (.x _returnvalue) (* _index _cellsize)))
      (`KismetSystemLibrary.DrawDebugLine` (`KismetMathLibrary.MakeVector` _returnvalue_2 (.y _returnvalue) (.z _returnvalue)) (`KismetMathLibrary.MakeVector` _returnvalue_2 (+ (.y _returnvalue) (* _gridextenty _cellsize)) (.z _returnvalue)) _linearcolor 999999.0 2.0))
    (for _index_2 (range (+ (- (+ _gridextenty 1) 1) 1))
      (bind _returnvalue_3 (+ (.y _returnvalue) (* _index_2 _cellsize)))
      (`KismetSystemLibrary.DrawDebugLine` (`KismetMathLibrary.MakeVector` (.x _returnvalue) _returnvalue_3 (.z _returnvalue)) (`KismetMathLibrary.MakeVector` (+ (.x _returnvalue) (* _gridextentx _cellsize)) _returnvalue_3 (.z _returnvalue)) _linearcolor 999999.0 2.0))))

(fn `DrawGrid`
  (bind _returnvalue (`self.K2_GetActorLocation`))
  (bind _linearcolor (make `LinearColor` 1.0 1.0 1.0 1.0))
  (bind _cellsize (`self.CellSize`))
  (bind _gridextentx (`self.GridExtentX`))
  (bind _gridextenty (`self.GridExtentY`))
  (if (`self.bShowGridInGame`)
    (for _index (range (+ (- (+ _gridextentx 1) 1) 1))
      (for _index_2 (range (+ (- _gridextenty 1) 1))
        (bind _returnvalue_2 (+ (.x _returnvalue) (* _index _cellsize)))
        (bind _returnvalue_3 (+ (.y _returnvalue) (* _index_2 _cellsize)))
        (bind _height (`self.SampleGroundHeight` _returnvalue_2 _returnvalue_3))
        (bind _returnvalue_4 (+ (.y _returnvalue) (* (+ _index_2 1) _cellsize)))
        (bind _height_2 (`self.SampleGroundHeight` _returnvalue_2 _returnvalue_4))
        (`KismetSystemLibrary.DrawDebugLine` (`KismetMathLibrary.MakeVector` _returnvalue_2 _returnvalue_3 (+ _height 5.0)) (`KismetMathLibrary.MakeVector` _returnvalue_2 _returnvalue_4 (+ _height_2 5.0)) _linearcolor 999999.0 2.0)))
    (for _index_3 (range (+ (- (+ _gridextenty 1) 1) 1))
      (for _index_4 (range (+ (- _gridextentx 1) 1))
        (bind _returnvalue_5 (+ (.x _returnvalue) (* _index_4 _cellsize)))
        (bind _returnvalue_6 (+ (.y _returnvalue) (* _index_3 _cellsize)))
        (bind _height_3 (`self.SampleGroundHeight` _returnvalue_5 _returnvalue_6))
        (bind _returnvalue_7 (+ (.x _returnvalue) (* (+ _index_4 1) _cellsize)))
        (bind _height_4 (`self.SampleGroundHeight` _returnvalue_7 _returnvalue_6))
        (`KismetSystemLibrary.DrawDebugLine` (`KismetMathLibrary.MakeVector` _returnvalue_5 _returnvalue_6 (+ _height_3 5.0)) (`KismetMathLibrary.MakeVector` _returnvalue_7 _returnvalue_6 (+ _height_4 5.0)) _linearcolor 999999.0 2.0)))))

(fn `GridCoordToWorld`
  (params (GridX :type Integer) (GridY :type Integer))
  (returns (WorldLocation :type "Vector Structure"))
  (bind _returnvalue (`self.K2_GetActorLocation`))
  (bind _cellsize (`self.CellSize`))
  (bind _returnvalue_2 (/ _cellsize 2.0))
  (return (`KismetMathLibrary.MakeVector` (+ (.x _returnvalue) (+ (* GridX _cellsize) _returnvalue_2)) (+ (.y _returnvalue) (+ (* GridY _cellsize) _returnvalue_2)) (.z _returnvalue))))

(fn `IsCellOccupied`
  (params (GridX :type Integer) (GridY :type Integer))
  (returns (bOccupied :type Boolean))
  (bind _key (`self.MakeCellKey` GridX GridY))
  (return (`BlueprintSetLibrary.Set_Contains` (`self.OccupiedCells`) _key)))

(fn `MakeCellKey`
  (params (GridX :type Integer) (GridY :type Integer))
  (returns (Key :type String))
  (return (`KismetStringLibrary.Concat_StrStr` (`KismetStringLibrary.Concat_StrStr` (`KismetStringLibrary.Conv_IntToString` GridX) ",") (`KismetStringLibrary.Conv_IntToString` GridY))))

(fn `SampleGroundHeight`
  (params (WorldX :type "Float (double-precision)") (WorldY :type "Float (double-precision)"))
  (returns (Height :type "Float (double-precision)"))
  (bind (_outhit _returnvalue) (`KismetSystemLibrary.LineTraceSingle` (`KismetMathLibrary.MakeVector` WorldX WorldY 20000.0) (`KismetMathLibrary.MakeVector` WorldX WorldY -5000.0) "TraceTypeQuery1" true))
  (if _returnvalue
    (return (.z (`.Location` (`GameplayStatics.BreakHitResult` _outhit))))
    (else
      (return 0.0))))

(fn `SetCellOccupied`
  (params (GridX :type Integer) (GridY :type Integer) (bOccupied :type Boolean))
  (bind _occupiedcells (`self.OccupiedCells`))
  (bind _key (`self.MakeCellKey` GridX GridY))
  (if bOccupied
    (`BlueprintSetLibrary.Set_Add` _occupiedcells _key)
    (else
      (`BlueprintSetLibrary.Set_Remove` _occupiedcells _key))))

(fn `UserConstructionScript`)

(fn `WorldToGridCoord`
  (params (WorldLocation :type "Vector Structure"))
  (returns (GridX :type Integer) (GridY :type Integer))
  (bind _returnvalue (`self.K2_GetActorLocation`))
  (bind _cellsize (`self.CellSize`))
  (return (`KismetMathLibrary.FFloor` (/ (- (.x WorldLocation) (.x _returnvalue)) _cellsize)) (`KismetMathLibrary.FFloor` (/ (- (.y WorldLocation) (.y _returnvalue)) _cellsize))))